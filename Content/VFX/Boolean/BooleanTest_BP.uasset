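; BooleanTest_BP is a test actor that feeds a sphere-shaped boolean volume into the material of its Sphere mesh.
; The construction script creates a dynamic material instance on Sphere and stores it as DMI.
; Every tick, it writes the Boolean sphere component's world location and scaled radius to the BooleanOrigin and BooleanRadius parameters, so the material follows that component as it moves or scales.
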(event `self.ReceiveTick`
  (params (DeltaSeconds :type "Float (single-precision)"))
  (bind _boolean (`self.Boolean`))
  (`MaterialInstanceDynamic.SetVectorParameterValue` (`self.DMI`) "BooleanOrigin" (`KismetMathLibrary.Conv_VectorToLinearColor` (`SceneComponent.K2_GetComponentLocation` _boolean)))
  (`MaterialInstanceDynamic.SetScalarParameterValue` (`self.DMI`) "BooleanRadius" (`SphereComponent.GetScaledSphereRadius` _boolean)))

(fn `UserConstructionScript`
  (bind _returnvalue (`PrimitiveComponent.CreateDynamicMaterialInstance` (`self.Sphere`) 0 null "None"))
  (set `self.DMI` _returnvalue))