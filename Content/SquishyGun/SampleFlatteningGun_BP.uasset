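; Sample gun actor that feeds wall-intersection data to its material, likely to flatten the gun mesh against surfaces it would clip into.
; BeginPlay creates a dynamic material instance on the Gun component.
; Each tick, a Visibility line trace runs from the gun along actor forward, with debug drawing.
; The result drives the material's intersect point (trace end on a miss), normal and hit flag, leaving any deformation to the shader.
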(event `self.ReceiveBeginPlay`
  (bind _gun (`self.Gun`))
  (bind _returnvalue (`PrimitiveComponent.CreateDynamicMaterialInstance` _gun 0 (`PrimitiveComponent.GetMaterial` _gun 0) "None"))
  (bind _output_get (set `self.MaterialInstance` _returnvalue))
  (`PrimitiveComponent.SetMaterial` _gun 0 _output_get))

(event `self.ReceiveTick`
  (params (DeltaSeconds :type "Float (single-precision)"))
  (bind _materialinstance (`self.MaterialInstance`))
  (bind _returnvalue (`SceneComponent.K2_GetComponentLocation` (`self.Gun`)))
  (bind (_outhit _returnvalue_2) (`KismetSystemLibrary.LineTraceSingle` :`Start` _returnvalue :`End` (+ _returnvalue (* (`self.GetActorForwardVector`) (`self.TraceLength`))) :`TraceChannel` "TraceTypeQuery1" :`DrawDebugType` "ForOneFrame"))
  (bind (_bblockinghit _binitialoverlap _time _distance _location _impactpoint _normal _impactnormal _physmat _hitactor _hitcomponent _hitbonename _bonename _hititem _elementindex _faceindex _tracestart _traceend) (`GameplayStatics.BreakHitResult` _outhit))
  (`MaterialInstanceDynamic.SetVectorParameterValue` _materialinstance "IntersectPoint" (`KismetMathLibrary.Conv_VectorToLinearColor` (`KismetMathLibrary.SelectVector` _impactpoint _traceend _returnvalue_2)))
  (`MaterialInstanceDynamic.SetScalarParameterValue` _materialinstance "Intersecting" (`KismetMathLibrary.SelectFloat` 1.0 0.0 _returnvalue_2))
  (`MaterialInstanceDynamic.SetVectorParameterValue` (`self.MaterialInstance`) "IntersectNormal" (`KismetMathLibrary.Conv_VectorToLinearColor` _impactnormal)))

(fn `UserConstructionScript`)